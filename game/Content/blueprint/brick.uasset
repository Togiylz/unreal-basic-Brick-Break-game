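; Breakable brick actor that loses one hitpoint each time it is hit by a ball.
; On BeginPlay it creates a Hitpoint widget, passes itself as the reference, and assigns it to its NumberWidget.
; The Hitbyball event calls Hitpointazaltma, which decrements Hitpoint or destroys the brick when it would reach zero, then plays an attack sound.
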(event `self.ReceiveBeginPlay`
  (bind _returnvalue (`|CreateWidget` "/Game/blueprint/hud/hitpoint.hitpoint_C"))
  (set `/Game/blueprint/hud/hitpoint.refbrick` self _returnvalue)
  (`WidgetComponent.SetWidget` (`self.numberWidget`) _returnvalue))

(event `/Game/blueprint/ballinterface.hitbyball`
  (`self.hitpointazaltma`)
  (`GameplayStatics.PlaySound2D` "/Game/audio_effects_retro/Animal_and_caracters/characters/attack/attack_variation.attack_variation" 1.0 1.0 0.0 null null))

(fn `hitpointazaltma`
  (if (<= (- (`self.hitpoint`) 1) 0)
    (`self.K2_DestroyActor`)
    (else
      (`/Engine/EditorBlueprintResources/StandardMacros.DecrementInt` (`self.hitpoint`)))))

(fn `UserConstructionScript`)
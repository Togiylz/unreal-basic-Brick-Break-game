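; Player-controlled bounce box (sektirmekutusu) that slides sideways along the world Y axis with mouse input.
; The mouse axis applies a swept world offset, only while the gamemodeball game mode's StadeOfTheGame matches one specific state.
; A separate Lifemecanic function decrements Life but never below one, with no handling for the last life and no caller in this graph.
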(event `InputAxis|mouse`
  (params (AxisValue :type "Float (single-precision)"))
  (bind _asgamemodeball (cast `/Game/blueprint/gamemodeball` (`GameplayStatics.GetGameMode`)))
  (if (`|EnumEquality` (`/Game/blueprint/gamemodeball.stade of the game` _asgamemodeball) "NewEnumerator5")
    (bind _output_get (set `self.Axis Value` AxisValue))
    (`self.K2_AddActorWorldOffset` (`KismetMathLibrary.MakeVector` 0.0 (* 10.0 _output_get)) true)))

(fn `lifemecanic`
  (if (not (<= (- (`self.life`) 1) 0))
    (`/Engine/EditorBlueprintResources/StandardMacros.DecrementInt` (`self.life`))))

(fn `UserConstructionScript`)